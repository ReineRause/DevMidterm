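; BP_Finish is the finish trigger of a timed maze.
; The first overlap with its box clears the timer held by the Begin actor, with no check on what entered.
; It then turns the light on every valid MazeFloor actor green and prints the completion time, derived by subtracting Begin's remaining Seconds from a hard-coded 30.
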(event OnComponentBeginOverlap(Box)
  (params (OverlappedComponent :type Primitive%20Component%20Object%20Reference) (OtherActor :type Actor%20Object%20Reference) (OtherComp :type Primitive%20Component%20Object%20Reference) (OtherBodyIndex :type Integer) (bFromSweep :type Boolean) (SweepResult :type Hit%20Result%20Structure%20%28by%20ref%29))
  (bind _begin (Variables|Default|GetBegin))
  (Utilities|FlowControl|DoOnce false
    (:Completed
      (Utilities|Time|ClearandInvalidateTimerbyHandle (Variables|/Game/ÖDEV/BP_Start.BP_Start_C|GetHandler _begin))
      (bind _outactors (Actor|GetAllActorsOfClass "/Game/ÖDEV/MazeFloor.MazeFloor_C"))
      (for _array_element _outactors
        (Utilities|IsValid (Variables|/Game/ÖDEV/MazeFloor.MazeFloor_C|GetLight _array_element)
          (:Is%20Valid
            (Rendering|Components|Light|SetLightColor (Variables|/Game/ÖDEV/MazeFloor.MazeFloor_C|GetLight _array_element) "(R=0.234243,G=1.000000,B=0.000000,A=1.000000)" true))))
      (Development|PrintString (Utilities|String|Append "Well done! Your time is" (Utilities|String|ToString(Float) (- 3e+01 (Variables|/Game/ÖDEV/BP_Start.BP_Start_C|GetSeconds _begin))) " SECONDS")))))

(fn ConstructionScript)