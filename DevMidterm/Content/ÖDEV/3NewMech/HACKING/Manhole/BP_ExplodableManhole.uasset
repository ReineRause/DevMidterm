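; Hackable manhole cover that explodes and launches upward when successfully hacked.
; Targeting events toggle a beam particle aimed at the player pawn and show a focus widget, whose progress-bar material tracks hacking progress.
; Success removes both components, spawns explosion effects and applies a randomized physics impulse.
; A random-spin timer is cleared immediately and on mesh hit; the Construction Script also calls the success event.
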(event OnComponentHit(ManholeMesh)
  (params (HitComponent :type Primitive%20Component%20Object%20Reference) (OtherActor :type Actor%20Object%20Reference) (OtherComp :type Primitive%20Component%20Object%20Reference) (NormalImpulse :type Vector :default "0, 0, 0") (Hit :type Hit%20Result%20Structure%20%28by%20ref%29))
  (Utilities|Time|ClearandInvalidateTimerbyHandle (stale EventOnSuccesfulHack _returnvalue_3))
  (Development|PrintString "ggg"))

(event Custom|Rotate%20Manhole
  (bind _returnvalue (Math|Random|RandomFloatinRange 1.0 5.0))
  (Transformation|AddLocalRotation (Variables|Default|GetManholeMesh) (Math|Rotator|MakeRotator _returnvalue _returnvalue _returnvalue) false false))

(event EventUpdateObjectHackingProgress
  (params (Progress%20Value :type Float%20%28double-precision%29))
  (bind _asfocused_object_ui (Utilities|Casting|CastToFocusedObject_UI (UserInterface|GetUserWidgetObject (Variables|Default|GetTargetedWidget))))
  (bind _returnvalue (Appearance|GetDynamicMaterial (Variables|/Game/ÖDEV/3NewMech/HACKING/Manhole/Visuals/FocusedObject_UI.FocusedObject_UI_C|GetProgressBar _asfocused_object_ui) :!class /Script/UMG.Image))
  (Class|Image|SetBrushfromMaterial (Variables|/Game/ÖDEV/3NewMech/HACKING/Manhole/Visuals/FocusedObject_UI.FocusedObject_UI_C|GetProgressBar _asfocused_object_ui) _returnvalue)
  (Rendering|Material|SetScalarParameterValue _returnvalue "Progress" Progress%20Value :!class /Script/Engine.MaterialInstanceDynamic))

(event EventOnSuccesfulHack
  (bind _returnvalue (Transformation|GetActorLocation))
  (bind _returnvalue_2 (Math|Random|RandomFloatinRange 5e+01 1.5e+02))
  (bind _manholemesh (Variables|Default|GetManholeMesh))
  (Components|DestroyComponent (Variables|Default|GetTargetedParticle))
  (Effects|SpawnEmitteratLocation "/Game/StarterContent/Particles/P_Explosion.P_Explosion" _returnvalue "0, 0, 0" "4.000000,4.000000,4.000000")
  (Audio|PlaySoundatLocation "/Game/StarterContent/Audio/Explosion_Cue.Explosion_Cue" _returnvalue "0, 0, 0" 1.0 1.0 0.0 0 0 0 0)
  (Physics|SetSimulatePhysics _manholemesh true)
  (Physics|AddImpulse _manholemesh (Math|Vector|MakeVector _returnvalue_2 _returnvalue_2 (Math|Random|RandomFloatinRange 7.5e+02 9.5e+02)) "None" true)
  (bind _returnvalue_3 (Utilities|Time|SetTimerbyEvent (delegate Custom|Rotate%20Manhole) 0.01))
  (Utilities|Time|ClearandInvalidateTimerbyHandle _returnvalue_3)
  (Development|PrintString "ggg"))

(event EventOnObjectTargeted
  (Rendering|SetVisibility (Variables|Default|GetTargetedWidget) true false)
  (Class|ParticleSystemComponent|SetBeamEndPoint (Variables|Default|GetTargetedParticle) 0 (Transformation|GetActorLocation (Pawn|GetControlledPawn (Game|GetPlayerController 0))))
  (Rendering|SetVisibility (Variables|Default|GetTargetedParticle) true false))

(event EventBeginPlay
  (Class|ParticleSystemComponent|SetBeamSourcePoint (Variables|Default|GetTargetedParticle) 1 (Transformation|GetWorldLocation (Variables|Default|GetManholeMesh)))
  (Development|PrintString "particle"))

(event EventOnObjectUnTargeted
  (Rendering|SetVisibility (Variables|Default|GetTargetedParticle) false false))

(fn ConstructionScript
  (CallFunction|OnSuccesfulHack))