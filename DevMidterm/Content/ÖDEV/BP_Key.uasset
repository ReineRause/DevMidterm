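; BP_Key is a key pickup that unlocks a linked Door actor.
; On Interract it sets the door's KeyFound flag to true and destroys itself.
; The construction script uses the Color enum to apply one of three materials to both the key mesh and the linked door's mesh, visually pairing them in the editor.
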(event EventBeginPlay)

(event Collision|EventActorBeginOverlap
  (params (OtherActor :type Actor%20Object%20Reference)))

(event EventTick
  (params (DeltaSeconds :type Float%20%28single-precision%29)))

(event EventInterract
  (Variables|/Game/ÖDEV/BP_Door.BP_Door_C|SetKey%20Found (Variables|Default|GetDoor) true)
  (Actor|DestroyActor))

(fn ConstructionScript
  (bind _staticmesh (Variables|Default|GetStaticMesh))
  (switch Utilities|FlowControl|Switch|Switchonbişeyler (Variables|Default|GetColor)
    (:NewEnumerator0
      (Rendering|Material|SetMaterial _staticmesh 0 "/Game/StarterContent/Materials/M_Brick_Cut_Stone.M_Brick_Cut_Stone"))
    (:NewEnumerator1
      (Rendering|Material|SetMaterial _staticmesh 0 "/Game/StarterContent/Props/Materials/M_Door.M_Door"))
    (:NewEnumerator2
      (Rendering|Material|SetMaterial _staticmesh 0 "/Game/StarterContent/Materials/M_Wood_Oak.M_Wood_Oak"))))