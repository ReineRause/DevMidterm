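; Gas trap actor that damages the player character standing inside its Box volume.
; Entering the box starts a non-looping timer that passes DotDamage to the character's HealthUpdate after DotTime; leaving clears it.
; On BeginPlay it binds to the character's DPTrap event through BindEventToDPTrap and destroys itself when the broadcast value matches its TrapType.
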(event OnComponentBeginOverlap(Box)
  (params (OverlappedComponent :type Primitive%20Component%20Object%20Reference) (OtherActor :type Actor%20Object%20Reference) (OtherComp :type Primitive%20Component%20Object%20Reference) (OtherBodyIndex :type Integer) (bFromSweep :type Boolean) (SweepResult :type Hit%20Result%20Structure%20%28by%20ref%29))
  (if (== OtherActor (Variables|Default|GetAs%20BP%20Third%20Person%20Character))
    (bind _returnvalue (Utilities|Time|SetTimerbyEvent (delegate Custom|Dot) (Variables|Default|Getdot%20time)))
    (Variables|Default|SetNewVar _returnvalue)))

(event OnComponentEndOverlap(Box)
  (params (OverlappedComponent :type Primitive%20Component%20Object%20Reference) (OtherActor :type Actor%20Object%20Reference) (OtherComp :type Primitive%20Component%20Object%20Reference) (OtherBodyIndex :type Integer))
  (if (== OtherActor (Variables|Default|GetAs%20BP%20Third%20Person%20Character))
    (Utilities|Time|ClearandInvalidateTimerbyHandle (Variables|Default|GetNewVar))))

(event Custom|Dot
  (Default|HealthUpdate (Variables|Default|GetAs%20BP%20Third%20Person%20Character) (Variables|Default|Getdot%20damage)))

(event Custom|Rah
  (params (NewParam :type TrapType%20Enum :default "NewEnumerator0"))
  (if (Utilities|Enum|Equal(Enum) NewParam (Variables|Default|GetTrap%20Type))
    (Actor|DestroyActor)))

(event EventBeginPlay
  (bind _asbp_third_person_character (Utilities|Casting|CastToBP_ThirdPersonCharacter (Game|GetPlayerCharacter 0)))
  (bind _output_get (Variables|Default|SetAs%20BP%20Third%20Person%20Character _asbp_third_person_character))
  (EventDispatchers|BindEventtoDPTrap _output_get (delegate Custom|Rah)))

(event Collision|EventActorBeginOverlap
  (params (OtherActor :type Actor%20Object%20Reference)))

(event EventTick
  (params (DeltaSeconds :type Float%20%28single-precision%29)))

(fn ConstructionScript)