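; BP_Disable is an interactable actor that signals the player character with its trap type, apparently to disable traps of that type.
; On BeginPlay it caches the player's BP_ThirdPersonCharacter and writes its TrapType enum name onto a TextRender label.
; Interract passes TrapType to the character's CallDPTrap, so this actor holds no trap references or disabling logic itself.
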(event EventBeginPlay
  (bind _asbp_third_person_character (Utilities|Casting|CastToBP_ThirdPersonCharacter (Game|GetPlayerCharacter 0)))
  (Variables|Default|SetAs%20BP%20Third%20Person%20Character _asbp_third_person_character)
  (Rendering|Components|TextRender|SetText (Variables|Default|GetTextRender) (Utilities|Text|ToText(String) (Utilities|String|EnumtoString (Variables|Default|GetTrapType)))))

(event Collision|EventActorBeginOverlap
  (params (OtherActor :type Actor%20Object%20Reference)))

(event EventTick
  (params (DeltaSeconds :type Float%20%28single-precision%29)))

(event EventInterract
  (Default|CallDPTrap (Variables|Default|GetAs%20BP%20Third%20Person%20Character) (Variables|Default|GetTrapType)))

(fn ConstructionScript)